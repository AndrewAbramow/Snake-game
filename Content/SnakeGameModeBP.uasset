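; Game mode for a Snake game that drives difficulty, level progression and win or lose transitions.
; Every tick it reads DataStorage from the game instance, applies hard-mode length and speed settings, and opens the lose level on EndGame.
; When the snake grows it calls CallIncrementFood.
; At max length it opens the win level if LevelCount equals MaxLevel, otherwise increments LevelCount, copies it into MaxLevel and loads 2_level.
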(event `self.ReceiveTick`
  (params (DeltaSeconds :type "Float (single-precision)"))
  (bind _snakelength (`self.SnakeLength`))
  ;[1 1 1] Hard difficulty
  (bind _asdata_storage (cast `/Game/DataStorage` (`GameplayStatics.GetGameInstance`)))
  (if (`/Game/DataStorage.IsHardLevel` _asdata_storage)
    (set `self.MaxLength` 20)
    (set `self.SpeedUpRate` 0.5)
    (set `self.SpeedUpRandom` 50))
  ;[1 1 1] Game Over
  (if (== true (`self.EndGame`))
    (`GameplayStatics.OpenLevel` "LoseLevel")
    (else
      ;[1 1 1] Nutrition
      (if (> _snakelength (`self.CurrentLength`))
        (set `self.CurrentLength` _snakelength)
        (`self.IncrementFood`)
        (if (== (`self.MaxLength`) _snakelength)
          (bind _levelcount (`/Game/DataStorage.LevelCount` _asdata_storage))
          ;[1 1 1] Win or nex level
          (if (== _levelcount (`/Game/DataStorage.Max_level` _asdata_storage))
            (`GameplayStatics.OpenLevel` "WinLevel")
            (else
              (bind _result (`/Engine/EditorBlueprintResources/StandardMacros.IncrementInt` _levelcount)
                (:`  `
                  (set `/Game/DataStorage.Max_level` _result _asdata_storage)
                  (`GameplayStatics.OpenLevel` "2_level"))))))))))

(fn `UserConstructionScript`)